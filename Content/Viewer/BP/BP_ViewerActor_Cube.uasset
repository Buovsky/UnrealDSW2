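; BP_ViewerActor_Cube is a viewer actor with a cube mesh whose visual effect can be switched on and off.
; Its OnEffect event flips the ActivatedEffectCube flag, swaps the Cube material between a clay brick material and the basic shape material, and prints the new state.
; BeginPlay, overlap and Tick are disabled stubs, and the construction script only calls its parent.
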(event `/Game/Viewer/BP/BPI_Effect.OnEffect`
  (if (`self.ActivatedEffectCube`)
    (`KismetSystemLibrary.PrintString` "Cube Effect - DEACTIVATED")
    (set `self.ActivatedEffectCube` false)
    (`PrimitiveComponent.SetMaterial` (`self.Cube`) 0 "/Engine/BasicShapes/BasicShapeMaterial.BasicShapeMaterial")
    (else
      (`KismetSystemLibrary.PrintString` "Cube Effect - ACTIVATED")
      (set `self.ActivatedEffectCube` true)
      (`PrimitiveComponent.SetMaterial` (`self.Cube`) 0 "/Game/StarterContent/Materials/M_Brick_Clay_New.M_Brick_Clay_New"))))

(fn `UserConstructionScript`
  (`parent.UserConstructionScript`))