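; BP_ViewerActor_Cone is a viewer actor with a toggleable "Cone Effect".
; Its OnEffect event flips the ActivatedEffectCone flag, prints the activated or deactivated state, and sets the Sphere component's visibility to match.
; BeginPlay, overlap and Tick are disabled stubs, and the construction script only calls its parent.
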(event `/Game/Viewer/BP/BPI_Effect.OnEffect`
  (if (`self.ActivatedEffectCone`)
    (`KismetSystemLibrary.PrintString` "Cone Effect - DEACTIVATED")
    (bind _output_get (set `self.ActivatedEffectCone` false))
    (`SceneComponent.SetVisibility` (`self.Sphere`) _output_get false)
    (else
      (`KismetSystemLibrary.PrintString` "Cone Effect - ACTIVATED")
      (bind _output_get_2 (set `self.ActivatedEffectCone` true))
      (`SceneComponent.SetVisibility` (`self.Sphere`) _output_get_2 false))))

(fn `UserConstructionScript`
  (`parent.UserConstructionScript`))